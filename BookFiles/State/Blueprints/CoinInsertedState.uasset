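; CoinInsertedState is the state of an old-school slot machine in which a casino coin has been inserted.
; It receives the machine reference through DoConstruction and handles its actions as part of a State pattern.
; Rejecting the coin switches the machine to its no-coin state, and pulling the lever switches it to the won-dollars state.
; Further inserts and payouts only print refusal messages, and restocking does nothing.
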(event EventBeginPlay)

(event Collision|EventActorBeginOverlap
  (params (OtherActor :type Actor%20Object%20Reference)))

(event EventTick
  (params (DeltaSeconds :type Float%20%28single-precision%29)))

(event EventInsertCoin
  (Development|PrintString "You cannot insert another casino coin" true true "(R=0.000000,G=0.660000,B=1.000000,A=1.000000)" 15.0))

(event EventRejectCoin
  (bind _oldschoolslotmachine (Variables|Default|GetoldSchoolSlotMachine))
  (Development|PrintString "Casino coin returned" true true "(R=0.000000,G=0.660000,B=1.000000,A=1.000000)" 15.0)
  (bind _nocoinstate (Default|GetNoCoinState _oldschoolslotmachine))
  (Default|SetState _oldschoolslotmachine _nocoinstate))

(event EventPullLever
  (bind _oldschoolslotmachine (Variables|Default|GetoldSchoolSlotMachine))
  (Development|PrintString "You pulled the lever..." true true "(R=0.000000,G=0.660000,B=1.000000,A=1.000000)" 15.0)
  (bind _wondollarsstate (Default|GetWonDollarsState _oldschoolslotmachine))
  (Default|SetState _oldschoolslotmachine _wondollarsstate))

(event EventPayout
  (Development|PrintString "No dollars dispensed" true true "(R=0.000000,G=0.660000,B=1.000000,A=1.000000)" 15.0))

(event EventRestockDollars)

(fn ConstructionScript)

(fn DoConstruction
  (params (oldSchoolSlotMachine :type Old%20School%20Slot%20Machine%20Object%20Reference))
  (Variables|Default|SetoldSchoolSlotMachine oldSchoolSlotMachine))