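; Concrete hotel builder in a Builder pattern example, filling a Lodging product with hotel descriptions for pool, lobby, restaurants and rooms.
; The construction script creates Lodging as a child actor, since spawning is unavailable there, and checks it for the FloorPlan interface.
; Each Build event sets one message through that interface, with restaurant and room setters swapped.
; GetLodging returns the product after the same interface check.
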(event EventBeginPlay)

(event Collision|EventActorBeginOverlap
  (params (OtherActor :type Actor%20Object%20Reference)))

(event EventBuildRooms
  ;[1 1 1] Custom Function check if lodging impelements interface
  (bind _lodging (CallFunction|IsLodingImplementInterface))
  (Class|FloorPlan|SetRestaurants(Message) _lodging "Luxury Suites"))

(event EventTick
  (params (DeltaSeconds :type Float%20%28single-precision%29)))

(event EventBuildSwimmingPool
  ;[1 1 1] Custom Function check if lodging impelements interface
  (bind _lodging (CallFunction|IsLodingImplementInterface))
  (Class|FloorPlan|SetSwimmingPool(Message) _lodging "Indoor Lagoon"))

(event EventBuildLobbyArea
  ;[1 1 1] Custom Function check if lodging impelements interface
  (bind _lodging (CallFunction|IsLodingImplementInterface))
  (Class|FloorPlan|SetLobbyArea(Message) _lodging "Grand Hall"))

(event EventBuildRestaurants
  ;[1 1 1] Custom Function check if lodging impelements interface
  (bind _lodging (CallFunction|IsLodingImplementInterface))
  (Class|FloorPlan|SetRooms(Message) _lodging "5 star Buffet"))

(fn ConstructionScript
  (bind _output_get (|Setlodging))
  (|lodgingisFloorPlan_int _output_get))

(fn IsLodingImplementInterface
  (bind _lodging (Variables|Default|Getlodging))
  (if (Utilities|DoesObjectImplementInterface _lodging "/Game/Builder/FloorPlan.FloorPlan_C")
    (return _lodging)))

(fn GetLodging
  (bind _lodging (Variables|Default|Getlodging))
  (if (Utilities|DoesObjectImplementInterface _lodging "/Game/Builder/FloorPlan.FloorPlan_C")
    (return _lodging)))