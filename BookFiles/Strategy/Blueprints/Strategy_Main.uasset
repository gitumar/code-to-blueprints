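; Demo driver actor for the Strategy design pattern, showing a battleship changing combat behavior at runtime.
; On BeginPlay it spawns a BruteForceStrategy actor and passes it into a newly spawned BattleShip.
; It then runs three scenarios in immediate succession, printing each threat and calling Engage on the same ship.
; Before the second and third, AlterManeuvers swaps in freshly spawned DivideConquer and Retreat strategy actors.
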(event EventBeginPlay
  (bind _returnvalue (|CreateBruteForceStrategy))
  (|CreateBattleship _returnvalue)
  (Utilities|FlowControl|Sequence
    (:then_0
      (|ExecuteBruteForceStrategy))
    (:then_1
      (|ExecuteDivideConquerStrategy))
    (:then_2
      (|ExecuteRetreatStrategy))))

(event Collision|EventActorBeginOverlap
  (params (OtherActor :type Actor%20Object%20Reference)))

(event EventTick
  (params (DeltaSeconds :type Float%20%28single-precision%29)))

(fn ConstructionScript)