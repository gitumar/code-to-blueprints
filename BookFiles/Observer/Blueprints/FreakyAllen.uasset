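; FreakyAllen is a subscriber in an Observer pattern example, reacting to time-of-day updates from a ClockTower publisher.
; Its construction script validates the ClockTower, checks that it implements the Publisher interface, then passes itself to SubscribeMessage.
; Update stores the received Time and calls Morph, which switches on morning, midday or evening to print that period's transformation message.
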(event EventBeginPlay)

(event Collision|EventActorBeginOverlap
  (params (OtherActor :type Actor%20Object%20Reference)))

(event EventTick
  (params (DeltaSeconds :type Float%20%28single-precision%29)))

(event EventUpdate
  (params (time :type String))
  (Variables|Default|Settime time)
  (CallFunction|Morph))

(event EventMorph
  (switch string (Variables|Default|Gettime)
    (:Morning
      (|Morning_Morph))
    (:Midday
      (|Midday_Morph))
    (:Evening
      (|Evening_Morph))))

(fn ConstructionScript
  (|isClockTowerValid
    (:Is%20Valid
      (|isClockTower_implement_Publisher_int
        (:then
          (|Subscribe_FreakyAllen_toClockTower)
          (|Print_Subscribe_Request))
        (:else
          (Development|PrintString "No"))))))