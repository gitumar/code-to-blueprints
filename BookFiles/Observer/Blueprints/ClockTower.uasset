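; ClockTower is the publisher in an Observer pattern example, holding a time of day and a list of subscribers.
; Objects register or leave through Subscribe and Unsubscribe events.
; SetTimeOfDay stores the new time and calls TimeChanged, which fires NotifySubscribers to send the time to each subscriber's UpdateMessage.
; A helper tests each subscriber for the Subscriber interface, but its result does not gate the message.
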(event EventBeginPlay)

(event Collision|EventActorBeginOverlap
  (params (OtherActor :type Actor%20Object%20Reference)))

(event EventTick
  (params (DeltaSeconds :type Float%20%28single-precision%29)))

(event EventSubscribe
  (params (s :type Actor%20Object%20Reference))
  (Utilities|Array|Add (Variables|Default|Getsubscribers) s))

(event EventUnsubscribe
  (params (s :type Actor%20Object%20Reference))
  (Utilities|Array|RemoveItem (Variables|Default|Getsubscribers) s))

(event EventNotifySubscribers
  (for _array_element (Variables|Default|Getsubscribers)
    (|isImplement_Subscriber_int _array_element)
    (Class|Subscriber|Update(Message) _array_element (Variables|Default|Gettime))))

(fn ConstructionScript)

(fn TimeChanged
  (CallFunction|NotifySubscribers))

(fn SetTimeOfDay
  (params (time :type String))
  (Variables|Default|Settime time)
  (CallFunction|TimeChanged))

(fn GetTime
  (return (Variables|Default|Gettime)))