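; Shooter is a Blueprint in an Adapter example that fires whatever slingshot object it is given through the SlingShot interface.
; The construction script checks that the assigned object is valid and implements the interface, then caches it in PrivSlingShot or prints a failure message.
; Sling rechecks the cached reference through a helper macro and calls SlingMessage on it, so Shooter relies only on the interface.
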(event EventBeginPlay)

(event Collision|EventActorBeginOverlap
  (params (OtherActor :type Actor%20Object%20Reference)))

(event EventTick
  (params (DeltaSeconds :type Float%20%28single-precision%29)))

(fn ConstructionScript
  (Utilities|IsValid (Variables|Default|GetslingShot)
    (:Is%20Valid
      (|isSlingShot_int
        (:then
          (Variables|Default|SetprivSlingShot (Variables|Default|GetslingShot)))
        (:else
          (Development|PrintString "No Hello"))))
    (:Is%20Not%20Valid
      (Development|PrintString "Not Valid"))))

(fn Sling
  (bind _privslingshot (|isSlingShot_int_1))
  (Class|SlingShot|Sling(Message) _privslingshot))