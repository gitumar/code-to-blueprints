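; Decorator-pattern enemy that wraps another Enemy actor to add a ranged gun attack, shown through printed text.
; The construction script stores DecoratedEnemy as the wrapped reference if it is valid and implements the Enemy interface, printing the outcome.
; Fight forwards to the wrapped enemy before printing its own attack line, and Die simply forwards.
; GetDamage adds a fixed bonus to the wrapped enemy's damage, layering behavior through interface calls.
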(event EventBeginPlay)

(event Collision|EventActorBeginOverlap
  (params (OtherActor :type Actor%20Object%20Reference)))

(event EventTick
  (params (DeltaSeconds :type Float%20%28single-precision%29)))

(event EventFight
  (Class|Enemy|Fight(Message) (Variables|Default|GetprivDecoratedEnemy))
  (Development|PrintString "The enemy blows a kiss and fires a gun" true true "(R=0.000000,G=0.660000,B=1.000000,A=1.000000)" 15.0))

(event EventDie
  (Class|Enemy|Die(Message) (Variables|Default|GetprivDecoratedEnemy)))

(fn ConstructionScript
  (bind _decoratedenemy (Variables|Default|GetdecoratedEnemy))
  (Utilities|IsValid _decoratedenemy
    (:Is%20Valid
      (if (Utilities|DoesObjectImplementInterface _decoratedenemy "/Game/Decorator/Enemy.Enemy_C")
        (bind _output_get (Variables|Default|SetprivDecoratedEnemy _decoratedenemy))
        (Development|PrintString (Utilities|String|Append (Utilities|GetDisplayName _output_get) " Implements Enemy") true true "(R=0.000000,G=0.660000,B=1.000000,A=1.000000)" 15.0)
        (else
          (Development|PrintString "No Hello"))))
    (:Is%20Not%20Valid
      (Development|PrintString "Not Valid"))))

(fn GetDamage
  (bind _damage (Class|Enemy|GetDamage(Message) (Variables|Default|GetprivDecoratedEnemy)))
  (return (+ _damage 95)))