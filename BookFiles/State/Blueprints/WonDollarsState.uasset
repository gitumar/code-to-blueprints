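; WonDollarsState is the state an old-school slot machine is in while paying out won dollars, as part of a State pattern.
; Coin and lever inputs only print rejection messages, and restocking does nothing.
; Payout has the machine emit dollars, then checks its remaining count to switch it to the NoCoin state, or to NoDollars when empty.
; DoConstruction stores the owning machine reference used for these calls.
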(event EventBeginPlay)

(event Collision|EventActorBeginOverlap
  (params (OtherActor :type Actor%20Object%20Reference)))

(event EventTick
  (params (DeltaSeconds :type Float%20%28single-precision%29)))

(event EventInsertCoin
  (Development|PrintString "Please wait, machine is dispensing dollars" true true "(R=0.000000,G=0.660000,B=1.000000,A=1.000000)" 15.0))

(event EventRejectCoin
  (Development|PrintString "Chill, you already pulled the lever" true true "(R=0.000000,G=0.660000,B=1.000000,A=1.000000)" 15.0))

(event EventPullLever
  (Development|PrintString "Do not pull lever twice!" true true "(R=0.000000,G=0.660000,B=1.000000,A=1.000000)" 15.0))

(event EventPayout
  (Default|EmitDollars (Variables|Default|GetoldSchoolSlotMachine))
  (|CheckMachineHasDollars
    (:then
      (|MachineHasDollars))
    (:else
      (|MachineOutofDollars))))

(event EventRestockDollars)

(fn ConstructionScript)

(fn DoConstruction
  (params (oldSchoolSlotMachine :type Old%20School%20Slot%20Machine%20Object%20Reference))
  (Variables|Default|SetoldSchoolSlotMachine oldSchoolSlotMachine))