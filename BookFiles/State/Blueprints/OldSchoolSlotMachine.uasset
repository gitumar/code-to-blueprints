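; Slot machine actor that implements the State design pattern, tracking a dollar count and a current state.
; The construction script spawns four state objects as child actors, gives each a reference to itself, then starts in NoCoin or NoDollars depending on the count.
; Coin, lever and restock actions forward messages to the current state through the State interface.
; Getters, SetState and EmitDollars expose transitions and fixed-amount payouts.
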(event EventBeginPlay)

(event Collision|EventActorBeginOverlap
  (params (OtherActor :type Actor%20Object%20Reference)))

(event EventTick
  (params (DeltaSeconds :type Float%20%28single-precision%29)))

(fn ConstructionScript
  (Utilities|FlowControl|Sequence
    (:then_0
      (|StateInitializations))
    (:then_1
      (Variables|Default|SetnumberOfDollars (Variables|Default|Getcount)))
    (:then_2
      (if (> (Variables|Default|GetnumberOfDollars) 0)
        (Variables|Default|Setstate (Variables|Default|GetnoCoinState))
        (else
          (Variables|Default|Setstate (Variables|Default|GetnoDollarsState)))))))

(fn InsertCoin
  (Class|State|InsertCoin(Message) (Variables|Default|Getstate)))

(fn RejectCoin
  (Class|State|RejectCoin(Message) (Variables|Default|Getstate)))

(fn PullLever
  (Class|State|PullLever(Message) (Variables|Default|Getstate))
  (Class|State|Payout(Message) (Variables|Default|Getstate)))

(fn EmitDollars
  (Development|PrintString "Make It Rain!" true true "(R=0.000000,G=0.660000,B=1.000000,A=1.000000)" 15.0)
  (if (!= (Variables|Default|Getcount) 0)
    (Variables|Default|Setcount (- (Variables|Default|Getcount) 50))))

(fn GetCount
  (return (Variables|Default|Getcount)))

(fn RestockDollars
  (params (count :type Integer))
  (Variables|Default|Setcount (+ count (Variables|Default|Getcount)))
  (Development|PrintString (Utilities|String|Append "The Old School Slot Machine was just filled and new dollar count is: " (Utilities|String|ToString(Integer) (Variables|Default|Getcount))) true true "(R=0.000000,G=0.660000,B=1.000000,A=1.000000)" 15.0)
  (Class|State|RestockDollars(Message) (Variables|Default|Getstate)))

(fn SetState
  (params (state :type Actor%20Object%20Reference))
  (Variables|Default|Setstate state))

(fn GetNoDollarsState
  (return (Variables|Default|GetnoDollarsState)))

(fn GetNoCoinState
  (return (Variables|Default|GetnoCoinState)))

(fn GetCoinInsertedState
  (return (Variables|Default|GetcoinInsertedState)))

(fn GetWonDollarsState
  (return (Variables|Default|GetwonDollarsState)))

(fn GetCurrentState
  (return (Utilities|String|Append "Current Slot Machine State: " (Utilities|GetDisplayName (Variables|Default|Getstate)))))

(fn InitNoDollarsState
  (bind _asno_dollars_state (|CreateNoDollarsState))
  (|isImplement_State_int_1 _asno_dollars_state)
  (bind _output_get (Variables|Default|SetnoDollarsState _asno_dollars_state))
  (Default|DoConstruction _output_get self))

(fn InitNoCoinState
  (bind _asno_coin_state (|CreateNoCoinState))
  (|isImplement_State_int_2 _asno_coin_state)
  (bind _output_get (Variables|Default|SetnoCoinState _asno_coin_state))
  (Default|DoConstruction _output_get self))

(fn InitCoinInsertedState
  (bind _ascoin_inserted_state (|CreateCoinInsertedState))
  (|isImplement_State_int _ascoin_inserted_state)
  (bind _output_get (Variables|Default|SetcoinInsertedState _ascoin_inserted_state))
  (Default|DoConstruction _output_get self))

(fn InitWonDollarsState
  (bind _aswon_dollars_state (|CreateWonDollarsState))
  (|isImplement_State_int_3 _aswon_dollars_state)
  (bind _output_get (Variables|Default|SetwonDollarsState _aswon_dollars_state))
  (Default|DoConstruction _output_get self))