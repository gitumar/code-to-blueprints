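; Singleton_Main is an actor that appears to demonstrate the Singleton pattern by attempting repeated Inventory spawns on BeginPlay.
; A fixed loop calls Create_Inventory_Instance, which spawns an Inventory actor and stores it in MyInventory when valid, otherwise hitting a delay.
; Instance_Created_Message prints the returned object's name as created, then delays.
; This graph never checks for an existing instance before spawning.
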(event EventBeginPlay
  (for _index (range 0 4)
    (bind _output_get (|Create_Inventory_Instance))
    (|Instance_Created_Message _output_get)))

(event Collision|EventActorBeginOverlap
  (params (OtherActor :type Actor%20Object%20Reference)))

(event EventTick
  (params (DeltaSeconds :type Float%20%28single-precision%29)))

(fn ConstructionScript)