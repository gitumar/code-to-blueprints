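; ArchitecturalEngineer is the director actor in a Builder pattern example, directing the construction of a lodging through an interchangeable builder.
; Its construction script checks that the supplied builder is valid and implements the LodgingBuilder interface, then stores it privately.
; ConstructLodging sends interface messages to build the pool, lobby, rooms and restaurants in fixed order, while GetLodging returns the builder's result.
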(event EventBeginPlay)

(event Collision|EventActorBeginOverlap
  (params (OtherActor :type Actor%20Object%20Reference)))

(event EventTick
  (params (DeltaSeconds :type Float%20%28single-precision%29)))

(fn ConstructionScript
  (bind _lodgingbuilder (Variables|Default|GetlodgingBuilder))
  (|ChecklodgingBuilderisValid _lodgingbuilder
    (:Is%20Valid
      (|lodgingBuilderisLodgingBuilder_int _lodgingbuilder)
      (Variables|Default|SetprivateLodgingBuilder _lodgingbuilder))))

(fn GetLodging
  (bind _privatelodgingbuilder (|isLodgingBuilder))
  (bind _lodging (Class|LodgingBuilder|GetLodging(Message) _privatelodgingbuilder))
  (return _lodging))

(fn ConstructLodging
  (Utilities|FlowControl|Sequence
    (:then_0
      (|buildSwimmingPool()))
    (:then_1
      (|buildLobbyArea()))
    (:then_2
      (|buildRooms()))
    (:then_3
      (|buildRestaurants()))))