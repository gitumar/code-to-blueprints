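; Driver actor for an Observer pattern example, wiring a ClockTower to a FreakyAllen that receives it on spawn.
; On BeginPlay it spawns and stores the ClockTower, then spawns FreakyAllen with that tower as a spawn parameter.
; It then sets the tower's time of day to morning, midday and evening in immediate succession to exercise the pattern.
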(event EventBeginPlay
  (bind _output_get (|CreateClockTower))
  (|CreateFreakyAllen _output_get)
  (Default|SetTimeOfDay (Variables|Default|GetclockTower) "Morning")
  (Default|SetTimeOfDay (Variables|Default|GetclockTower) "Midday")
  (Default|SetTimeOfDay (Variables|Default|GetclockTower) "Evening"))

(event Collision|EventActorBeginOverlap
  (params (OtherActor :type Actor%20Object%20Reference)))

(event EventTick
  (params (DeltaSeconds :type Float%20%28single-precision%29)))

(fn ConstructionScript)