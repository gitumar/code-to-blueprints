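; Adapter_Main is the driver actor for an Adapter pattern example, wiring a gun adapter into a shooter.
; On BeginPlay it spawns the gun adapter, then spawns a shooter with that adapter passed as its SlingShot.
; It stores the shooter and calls Sling on it, so the adapter stands in wherever the shooter expects a slingshot.
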(event EventBeginPlay
  (bind _returnvalue (|Create_Gun_Adapter))
  (bind _output_get (|Create_Shooter _returnvalue))
  (Default|Sling _output_get))

(event Collision|EventActorBeginOverlap
  (params (OtherActor :type Actor%20Object%20Reference)))

(event EventTick
  (params (DeltaSeconds :type Float%20%28single-precision%29)))

(fn ConstructionScript)