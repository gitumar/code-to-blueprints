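; State_Main is a demo driver that exercises the states of an OldSchoolSlotMachine.
; On BeginPlay it spawns the machine with an initial count, stores the reference and runs three scripted action sequences in order.
; The sequences mix coin inserts, lever pulls and a dollar restock, printing the machine's current state along the way to show how it responds.
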(event EventBeginPlay
  (|CreateOldSchoolSlotMachine)
  (Utilities|FlowControl|Sequence
    (:then_0
      (|OldSchoolSlotMachineActionSequence_1))
    (:then_1
      (|OldSchoolSlotMachineActionSequence_2))
    (:then_2
      (|OldSchoolSlotMachineActionSequence_3))))

(event Collision|EventActorBeginOverlap
  (params (OtherActor :type Actor%20Object%20Reference)))

(event EventTick
  (params (DeltaSeconds :type Float%20%28single-precision%29)))

(fn ConstructionScript)

(fn PrintCurrentState
  (bind _statestring (Default|GetCurrentState (Variables|Default|GetoldSchoolSlotMachine)))
  (Development|PrintString _statestring true true "(R=0.000000,G=0.660000,B=1.000000,A=1.000000)" 15.0))