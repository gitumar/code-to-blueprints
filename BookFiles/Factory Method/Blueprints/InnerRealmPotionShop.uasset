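; Inner Realm potion shop, a concrete creator in a Factory Method example that spawns Inner Realm variants of potions.
; Its ConcoctPotion override switches on the potion SKU to run one spawn graph each for Health, Power and Skill, printing an error for any other SKU.
; Each graph spawns its actor at Location and stores it in NewPotion, then the override calls the parent ConcoctPotion and returns NewPotion.
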(event EventBeginPlay
  (|CallParentFunction))

(event Collision|EventActorBeginOverlap
  (params (OtherActor :type Actor%20Object%20Reference))
  (|CallParentFunction OtherActor) ; This node is disabled and will not be called.\nDrag off pins to build functionality.
)

(event EventTick
  (params (DeltaSeconds :type Float%20%28single-precision%29))
  (|CallParentFunction DeltaSeconds) ; This node is disabled and will not be called.\nDrag off pins to build functionality.
)

(fn ConstructionScript
  (|CallParentFunction))

(fn ConcoctPotion
  (params (potionSKU :type String))
  (Utilities|FlowControl|Sequence
    (:then_0
      (switch string potionSKU
        (:Default
          (Development|PrintString "Unable to spawn Inner Realm Potions" true true "(R=0.000000,G=0.660000,B=1.000000,A=1.000000)" 15.0))
        (:Health
          (|New_InnerRealmHealthPotion))
        (:Power
          (|New_InnerRealmPowerPotion))
        (:Skill
          (|New_InnerRealmSkillPotion))))
    (:then_1
      (|CallParentFunction potionSKU)
      (return (Variables|Default|GetnewPotion)))))