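; PotionShop is a base shop Blueprint that takes potion orders, illustrating the Factory Method pattern.
; OrderPotion gets a potion from ConcoctPotion, stores it, prints its name, runs its boil, bubble, brew and bottle steps in order, then returns it.
; ConcoctPotion is an empty factory hook, leaving the choice of concrete potion to child shops while the ordering sequence stays shared.
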(event EventBeginPlay
  (|CallParentFunction) ; This node is disabled and will not be called.\nDrag off pins to build functionality.
)

(event Collision|EventActorBeginOverlap
  (params (OtherActor :type Actor%20Object%20Reference))
  (|CallParentFunction OtherActor) ; This node is disabled and will not be called.\nDrag off pins to build functionality.
)

(event EventTick
  (params (DeltaSeconds :type Float%20%28single-precision%29))
  (|CallParentFunction DeltaSeconds) ; This node is disabled and will not be called.\nDrag off pins to build functionality.
)

(fn ConstructionScript
  (|CallParentFunction))

(fn ConcoctPotion
  (params (potionSKU :type String))
  (return 0))

(fn OrderPotion
  (params (category :type String))
  (|Set_Concocting_Potion category)
  (Utilities|FlowControl|Sequence
    (:then_0
      (|Print_Concocting_Potion_Name))
    (:then_1
      (|Boil_Potion))
    (:then_2
      (|Bubble_Potion))
    (:then_3
      (|Brew_Potion))
    (:then_4
      (|Bottle_Potion))
    (:then_5
      (return (Variables|Default|Getpotion)))))