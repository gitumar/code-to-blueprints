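; Lodging is an Actor Blueprint that acts as the product in a Builder example, representing a lodging made of separate parts.
; Four setter events store the swimming pool, lobby area, rooms and restaurants, and each prints the value it receives.
; It holds no assembly logic of its own, as the construction script is empty and the default events are disabled.
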(event EventBeginPlay)

(event Collision|EventActorBeginOverlap
  (params (OtherActor :type Actor%20Object%20Reference)))

(event EventSetRestaurants
  (params (restaurants :type String))
  (bind _output_get (Variables|Default|Setrestaurants restaurants))
  (Development|PrintString _output_get true true "(R=0.000000,G=0.660000,B=1.000000,A=1.000000)" 1e+01))

(event EventTick
  (params (DeltaSeconds :type Float%20%28single-precision%29)))

(event EventSetSwimmingPool
  (params (swimmingPool :type String))
  (bind _output_get (Variables|Default|SetswimmingPool swimmingPool))
  (Development|PrintString _output_get true true "(R=0.000000,G=0.660000,B=1.000000,A=1.000000)" 1e+01))

(event EventSetLobbyArea
  (params (lobbyArea :type String))
  (bind _output_get (Variables|Default|SetlobbyArea lobbyArea))
  (Development|PrintString _output_get true true "(R=0.000000,G=0.660000,B=1.000000,A=1.000000)" 1e+01))

(event EventSetRooms
  (params (rooms :type String))
  (bind _output_get (Variables|Default|Setrooms rooms))
  (Development|PrintString _output_get true true "(R=0.000000,G=0.660000,B=1.000000,A=1.000000)" 1e+01))

(fn ConstructionScript)