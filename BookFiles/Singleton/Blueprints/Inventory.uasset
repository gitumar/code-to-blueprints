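; Inventory actor Blueprint that enforces a singleton, allowing one instance in the level; it holds no inventory logic.
; The Construction Script uses GetAllActorsOfClass to check whether more than one Inventory actor exists and takes the first one found.
; If so, it prints that actor's display name with an "already exists" message and destroys itself.
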(event EventBeginPlay)

(event Collision|EventActorBeginOverlap
  (params (OtherActor :type Actor%20Object%20Reference)))

(event EventTick
  (params (DeltaSeconds :type Float%20%28single-precision%29)))

(fn ConstructionScript
  (bind (_returnvalue _output) (|isInstance_already_exist))
  (if _returnvalue
    (bind _output_get (Variables|Default|SetInstance _output))
    (|kill_yourself _output_get)))