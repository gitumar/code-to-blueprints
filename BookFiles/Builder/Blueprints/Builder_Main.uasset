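; Demo actor that runs the Builder pattern on BeginPlay to construct a hotel lodging.
; It spawns a HotelLodgingBuilder and passes it to a spawned ArchitecturalEngineer, which acts as director and constructs the lodging.
; It then retrieves the lodging from the engineer, checks that it implements the FloorPlan interface, and prints whether the hotel was built.
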(event EventBeginPlay
  (Utilities|FlowControl|Sequence
    (:then_0
      (bind _output_get (|SethotelBuilder))
      (bind _output_get_2 (|Setengineer _output_get))
      (Default|ConstructLodging _output_get_2))
    (:then_1
      (bind _output_get_3 (|Setlodging))
      (|lodgingisFloorPlan_int _output_get_3
        (:then
          (Development|PrintString "Built a Hotel" true true "(R=0.000000,G=0.660000,B=1.000000,A=1.000000)" 2e+01))
        (:else
          (Development|PrintString "Failed to Build a Hotel" true true "(R=0.000000,G=0.660000,B=1.000000,A=1.000000)" 2e+01))))))

(event Collision|EventActorBeginOverlap
  (params (OtherActor :type Actor%20Object%20Reference)))

(event EventTick
  (params (DeltaSeconds :type Float%20%28single-precision%29)))

(fn ConstructionScript)