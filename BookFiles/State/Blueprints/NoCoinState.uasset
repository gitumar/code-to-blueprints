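; NoCoinState is the state of an old-school slot machine that has no coin inserted, part of a State pattern implementation.
; InsertCoin prints a confirmation and switches the machine to its CoinInserted state through the reference stored by DoConstruction.
; RejectCoin, PullLever and Payout only print messages refusing the action, and RestockDollars does nothing.
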(event EventBeginPlay)

(event Collision|EventActorBeginOverlap
  (params (OtherActor :type Actor%20Object%20Reference)))

(event EventTick
  (params (DeltaSeconds :type Float%20%28single-precision%29)))

(event EventInsertCoin
  (Development|PrintString "You inserted a casino coin" true true "(R=0.000000,G=0.660000,B=1.000000,A=1.000000)" 15.0)
  (bind _coininsertedstate (Default|GetCoinInsertedState (Variables|Default|GetoldSchoolSlotMachine)))
  (Default|SetState (Variables|Default|GetoldSchoolSlotMachine) _coininsertedstate))

(event EventRejectCoin
  (Development|PrintString "You haven't inserted a casino coin" true true "(R=0.000000,G=0.660000,B=1.000000,A=1.000000)" 15.0))

(event EventPullLever
  (Development|PrintString "You turned, but there's no casino coin" true true "(R=0.000000,G=0.660000,B=1.000000,A=1.000000)" 15.0))

(event EventPayout
  (Development|PrintString "You need to pay first" true true "(R=0.000000,G=0.660000,B=1.000000,A=1.000000)" 15.0))

(event EventRestockDollars)

(fn ConstructionScript)

(fn DoConstruction
  (params (oldSchoolSlotMachine :type Old%20School%20Slot%20Machine%20Object%20Reference))
  (Variables|Default|SetoldSchoolSlotMachine oldSchoolSlotMachine))