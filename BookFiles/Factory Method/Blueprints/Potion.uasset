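; Potion actor Blueprint, the product in a Factory Method pattern example, modeling the preparation steps of a named potion.
; Boil, Bubble, Brew and Bottle are separate functions that only print placeholder messages, with Boil including the PotionName and its ingredients.
; GetPotionName exposes the name, while the event graph and construction script hold no logic, so the steps rely on external callers.
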(event EventBeginPlay)

(event Collision|EventActorBeginOverlap
  (params (OtherActor :type Actor%20Object%20Reference)))

(event EventTick
  (params (DeltaSeconds :type Float%20%28single-precision%29)))

(fn ConstructionScript)

(fn Boil
  (Utilities|FlowControl|Sequence
    (:then_0
      (Development|PrintString (Utilities|String|Append "Boil " (Variables|Default|GetpotionName)) true true "(R=0.000000,G=0.660000,B=1.000000,A=1.000000)" 15.0))
    (:then_1
      (Development|PrintString "Drop in blood..." true true "(R=0.000000,G=0.660000,B=1.000000,A=1.000000)" 15.0))
    (:then_2
      (Development|PrintString "Drop in herbs.." true true "(R=0.000000,G=0.660000,B=1.000000,A=1.000000)" 15.0))))

(fn Bubble
  (Development|PrintString "Bubble for 3 moons and a sunset" true true "(R=0.000000,G=0.660000,B=1.000000,A=1.000000)" 15.0))

(fn Brew
  (Development|PrintString "Brewing at Low Temperature" true true "(R=0.000000,G=0.660000,B=1.000000,A=1.000000)" 15.0))

(fn Bottle
  (Development|PrintString "Bottle concoction in flask" true true "(R=0.000000,G=0.660000,B=1.000000,A=1.000000)" 15.0))

(fn GetPotionName
  (return (Variables|Default|GetpotionName)))