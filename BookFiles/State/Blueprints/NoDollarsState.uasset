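; NoDollarsState is the out-of-money state of an old-school slot machine, built with the State pattern.
; It responds to coin insert, coin reject, lever pull and payout events only by printing a message.
; RestockDollars switches the machine to its NoCoin state through SetState.
; DoConstruction stores the owning OldSchoolSlotMachine reference used for that transition.
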(event EventBeginPlay)

(event Collision|EventActorBeginOverlap
  (params (OtherActor :type Actor%20Object%20Reference)))

(event EventTick
  (params (DeltaSeconds :type Float%20%28single-precision%29)))

(event EventInsertCoin
  (Development|PrintString "You cannot insert a casino coin, the machine is out of money" true true "(R=0.000000,G=0.660000,B=1.000000,A=1.000000)" 15.0))

(event EventRejectCoin
  (Development|PrintString "You have not inserted a casino coin" true true "(R=0.000000,G=0.660000,B=1.000000,A=1.000000)" 15.0))

(event EventPullLever
  (Development|PrintString "You turned, but there is NO money in the machine" true true "(R=0.000000,G=0.660000,B=1.000000,A=1.000000)" 15.0))

(event EventPayout
  (Development|PrintString "No money was paid out" true true "(R=0.000000,G=0.660000,B=1.000000,A=1.000000)" 15.0))

(event EventRestockDollars
  (bind _oldschoolslotmachine (Variables|Default|GetoldSchoolSlotMachine))
  (bind _nocoinstate (Default|GetNoCoinState _oldschoolslotmachine))
  (Default|SetState _oldschoolslotmachine _nocoinstate))

(fn ConstructionScript)

(fn DoConstruction
  (params (oldSchoolSlotMachine :type Old%20School%20Slot%20Machine%20Object%20Reference))
  (Variables|Default|SetoldSchoolSlotMachine oldSchoolSlotMachine))