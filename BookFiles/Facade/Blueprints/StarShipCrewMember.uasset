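; StarShipCrewMember is a crew member Blueprint in a Facade pattern example, carrying out shipboard routine tasks.
; TaskPerform loops over a task list and passes each to Task, which switches to lights out, trice up, liberty call, muster or duty.
; The routine calls print announcements prefixed by CrewTitle.
; CrewTitle returns an empty string and Duty does nothing, leaving both as apparent override points for specific crew roles.
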(event EventBeginPlay)

(event Collision|EventActorBeginOverlap
  (params (OtherActor :type Actor%20Object%20Reference)))

(event EventTick
  (params (DeltaSeconds :type Float%20%28single-precision%29)))

(fn ConstructionScript)

(fn TurnLightsOut
  (bind _crewtitle (CallFunction|CrewTitle))
  (Development|PrintString (Utilities|String|Append _crewtitle " taps,taps lights out.") true true "(R=0.000000,G=0.660000,B=1.000000,A=1.000000)" 15.0))

(fn HeaveOutTriceUp
  (bind _crewtitle (CallFunction|CrewTitle))
  (Development|PrintString (Utilities|String|Append _crewtitle " all hands heave out and trice up.") true true "(R=0.000000,G=0.660000,B=1.000000,A=1.000000)" 15.0))

(fn LibertyCall
  (bind _crewtitle (CallFunction|CrewTitle))
  (Development|PrintString (Utilities|String|Append _crewtitle " liberty call, liberty call.") true true "(R=0.000000,G=0.660000,B=1.000000,A=1.000000)" 15.0))

(fn CrewMuster
  (bind _crewtitle (CallFunction|CrewTitle))
  (Development|PrintString (Utilities|String|Append _crewtitle " time for muster.") true true "(R=0.000000,G=0.660000,B=1.000000,A=1.000000)" 15.0))

(fn Task
  (params (task :type String))
  (switch string task
    (:Default
      (Development|PrintString "Undefined task" true true "(R=0.000000,G=0.660000,B=1.000000,A=1.000000)" 15.0))
    (:lights_out
      (CallFunction|TurnLightsOut))
    (:trice_up
      (CallFunction|HeaveOutTriceUp))
    (:liberty_call
      (CallFunction|LibertyCall))
    (:muster
      (CallFunction|CrewMuster))
    (:duty
      (CallFunction|Duty))))

(fn TaskPerform
  (params (tasks :type Array%20of%20Strings))
  (for _array_element tasks
    (CallFunction|Task _array_element)))

(fn Duty)

(fn CrewTitle
  (return ""))