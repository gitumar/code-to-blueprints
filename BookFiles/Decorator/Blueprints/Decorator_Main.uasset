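; Demo actor for the Decorator pattern that shows a base melee enemy and a projectile enemy that decorates it.
; On BeginPlay it spawns a MeleeEnemy, then a ProjectileEnemy that receives the melee instance as its DecoratedEnemy.
; Each enemy in turn gets fight, die and damage calls through small wrapper functions, with the returned damage printed to screen.
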(event EventBeginPlay
  (Development|PrintString "Melee Enemies are on the horizon" true true "(R=0.000000,G=0.660000,B=1.000000,A=1.000000)" 15.0)
  (Utilities|FlowControl|Sequence
    (:then_0
      (|Melee_Enemy_Actions))
    (:then_1
      (|Projectile_Enemy_Actions))))

(event Collision|EventActorBeginOverlap
  (params (OtherActor :type Actor%20Object%20Reference)))

(event EventTick
  (params (DeltaSeconds :type Float%20%28single-precision%29)))

(fn ConstructionScript)