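; StarShipFacade is an actor demonstrating the Facade pattern, giving simple daily-routine calls over a starship crew of officers.
; On BeginPlay it spawns Navigation, Supply and Operations officers and adds them to the Crew array.
; Reveille, PlanOfTheDay and Taps each rebuild the Tasks list with named duties, then PerformTasks passes it to every crew member's TaskPerform.
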(event EventBeginPlay
  (Utilities|FlowControl|Sequence
    (:then_0
      (|AddNavigationOfficertocrew))
    (:then_1
      (|AddSupplyOfficertocrew))
    (:then_2
      (|AddOperationsOfficertoCrew))))

(event Collision|EventActorBeginOverlap
  (params (OtherActor :type Actor%20Object%20Reference)))

(event EventTick
  (params (DeltaSeconds :type Float%20%28single-precision%29)))

(fn ConstructionScript)

(fn Reveille
  (bind _tasks (Variables|Default|Gettasks))
  (Utilities|Array|Clear _tasks)
  (Utilities|Array|Add _tasks "trice_up")
  (Utilities|Array|Add _tasks "muster")
  (CallFunction|PerformTasks (Variables|Default|Getcrew) (Variables|Default|Gettasks)))

(fn PlanOftheDay
  (bind _tasks (Variables|Default|Gettasks))
  (Utilities|Array|Clear _tasks)
  (Utilities|Array|Add _tasks "duty")
  (CallFunction|PerformTasks (Variables|Default|Getcrew) (Variables|Default|Gettasks)))

(fn Taps
  (bind _tasks (Variables|Default|Gettasks))
  (Utilities|Array|Clear _tasks)
  (Utilities|Array|Add _tasks "liberty_call")
  (Utilities|Array|Add _tasks "lights_out")
  (CallFunction|PerformTasks (Variables|Default|Getcrew) (Variables|Default|Gettasks)))

(fn PerformTasks
  (params (crew :type Array%20of%20Star%20Ship%20Crew%20Member%20Object%20References) (tasks :type Array%20of%20Strings))
  (for _array_element crew
    (Default|TaskPerform _array_element tasks)))