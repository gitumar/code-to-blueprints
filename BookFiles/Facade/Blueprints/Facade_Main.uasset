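; Facade_Main is a demo actor for the Facade pattern, driving a starship's daily routine through a single facade object.
; On BeginPlay, Create_Starship_Facade spawns a StarShipFacade at the Location transform and stores it in ShipFacade.
; A sequence then calls Reveille, PlanOfTheDay and Taps on that reference in order, leaving their implementation to the facade.
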(event EventBeginPlay
  (|Create_Starship_Facade)
  (Utilities|FlowControl|Sequence
    (:then_0
      (Default|Reveille (Variables|Default|GetshipFacade)))
    (:then_1
      (Default|PlanOftheDay (Variables|Default|GetshipFacade)))
    (:then_2
      (Default|Taps (Variables|Default|GetshipFacade)))))

(event Collision|EventActorBeginOverlap
  (params (OtherActor :type Actor%20Object%20Reference)))

(event EventTick
  (params (DeltaSeconds :type Float%20%28single-precision%29)))

(fn ConstructionScript)