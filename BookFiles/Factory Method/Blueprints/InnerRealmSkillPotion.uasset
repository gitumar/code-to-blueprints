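; InnerRealmSkillPotion is a concrete potion product in a Factory Method example, representing the Inner Realm skill potion.
; Its construction script calls the parent's, then sets the potion name, gooeyness and blood type and adds Inner Realm herbs to the Herbs array.
; The Brew event only prints a high-temperature brewing message, and the BeginPlay, overlap and Tick events are disabled.
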(event EventBeginPlay
  (|CallParentFunction) ; This node is disabled and will not be called.\nDrag off pins to build functionality.
)

(event Collision|EventActorBeginOverlap
  (params (OtherActor :type Actor%20Object%20Reference))
  (|CallParentFunction OtherActor) ; This node is disabled and will not be called.\nDrag off pins to build functionality.
)

(event EventTick
  (params (DeltaSeconds :type Float%20%28single-precision%29))
  (|CallParentFunction DeltaSeconds) ; This node is disabled and will not be called.\nDrag off pins to build functionality.
)

(event EventBrew
  (Development|PrintString "Brewing at High Temperature" true true "(R=0.000000,G=0.660000,B=1.000000,A=1.000000)" 15.0))

(fn ConstructionScript
  (|CallParentFunction)
  (Utilities|FlowControl|Sequence
    (:then_0
      (Variables|Default|SetpotionName "Inner Realm Skill Potion"))
    (:then_1
      (Variables|Default|Setgooeyness "Mucus Like"))
    (:then_2
      (Variables|Default|Setblood "Orc Blood"))
    (:then_3
      (Utilities|Array|Add (Variables|Default|Getherbs) "Root of Inner Realm"))
    (:then_4
      (Utilities|Array|Add (Variables|Default|Getherbs) "Sage of Inner Realm"))
    (:then_5
      (Utilities|Array|Add (Variables|Default|Getherbs) "Wildrose of Inner Realm"))
    (:then_6
      (Utilities|Array|Add (Variables|Default|Getherbs) "Yarrow of Inner Realm"))))