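; BattleShip is an actor that demonstrates the Strategy pattern by delegating its maneuver to a swappable strategy object.
; The construction script uses validity and interface-check macros to store an assigned BattleStrategy implementing BattleShipStrategy, printing the result.
; AlterManeuvers repeats those checks inline to swap the stored strategy at runtime.
; Engage calls ManeuverMessage on the stored strategy without checking it.
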(event EventBeginPlay)

(event Collision|EventActorBeginOverlap
  (params (OtherActor :type Actor%20Object%20Reference)))

(event EventTick
  (params (DeltaSeconds :type Float%20%28single-precision%29)))

(fn ConstructionScript
  (bind _battlestrategy (Variables|Default|GetbattleStrategy))
  (|isVailid _battlestrategy
    (:Is%20Valid
      (|isImplementBattleShipStrategy_int _battlestrategy
        (:then
          (bind _output_get (Variables|Default|SetprivBattleStrategy (Variables|Default|GetbattleStrategy)))
          (|PrintBattleStrategy _output_get))
        (:else
          (Development|PrintString "No"))))))

(fn AlterManeuvers
  (params (battleStrategy :type Actor%20Object%20Reference))
  (bind _output_get (Variables|Default|SetbattleStrategy battleStrategy))
  (Utilities|IsValid _output_get
    (:Is%20Valid
      (if (Utilities|DoesObjectImplementInterface _output_get "/Game/Strategy/BattleShipStrategy.BattleShipStrategy_C")
        (bind _output_get_2 (Variables|Default|SetprivBattleStrategy _output_get))
        (Development|PrintString (Utilities|String|Append (Utilities|GetDisplayName _output_get_2) " Implements BattleStrategy") true true "(R=0.000000,G=0.660000,B=1.000000,A=1.000000)" 15.0)
        (else
          (Development|PrintString "No Hello" true true "(R=0.000000,G=0.660000,B=1.000000,A=1.000000)" 15.0))))
    (:Is%20Not%20Valid
      (Development|PrintString "Not Valid"))))

(fn Engage
  (Class|BattleShipStrategy|Maneuver(Message) (Variables|Default|GetprivBattleStrategy)))