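; Demo driver actor for the Factory Method pattern, using an Inner Realm potion shop.
; On BeginPlay it spawns an InnerRealmPotionShop and stores it, then orders Health, Power and Skill potions in sequence.
; Each order calls the shop's OrderPotion with a type string, so this Blueprint only requests potions and leaves their creation to the shop.
; Each returned potion's name is printed to the screen.
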(event EventBeginPlay
  (|Spawn_Inner_Realm_Shop)
  (|Enter_Inner_Realm_Potion_Shop))

(event Collision|EventActorBeginOverlap
  (params (OtherActor :type Actor%20Object%20Reference)))

(event EventTick
  (params (DeltaSeconds :type Float%20%28single-precision%29)))

(fn ConstructionScript)

(fn PrintPotionInfo
  (params (B :type String))
  (Development|PrintString (Utilities|String|Append "Potion is " B) true true "(R=0.000000,G=0.660000,B=1.000000,A=1.000000)" 15.0))